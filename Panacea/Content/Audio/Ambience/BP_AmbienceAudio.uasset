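; BP_AmbienceAudio controls the ambient soundscape through three audio components: wind, rain/cricket and music.
; A start event plays all three from the beginning.
; Separate events fade the music, or the wind and rain/cricket layers as a pair, in and out using shared fade durations.
; Another event passes a DistortionAmount float parameter to the music source to drive distortion at runtime.
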(event Custom|MusicDistortionAmount_Event
  (params (DistortionAmount :type Float%20%28double-precision%29))
  (Audio|Parameter|SetFloatParameter (Variables|Default|GetMSS_Music) "DistortionAmount" DistortionAmount :!class /Script/Engine.AudioComponent))

(event Custom|StopAmbienceSounds_Event
  (bind _fadeoutduration (Variables|Default|GetFadeoutDuration))
  (Audio|Components|Audio|FadeOut (Variables|Default|GetMSS_Rain_Cricket) _fadeoutduration 0.0 "Linear" :!class /Script/Engine.AudioComponent)
  (Audio|Components|Audio|FadeOut (Variables|Default|GetMSS_Wind) _fadeoutduration 0.0 "Linear" :!class /Script/Engine.AudioComponent))

(event Custom|StartPlayingSound
  (Audio|Components|Audio|Play (Variables|Default|GetMSS_Wind) 0.0)
  (Audio|Components|Audio|Play (Variables|Default|GetMSS_Rain_Cricket) 0.0)
  (Audio|Components|Audio|Play (Variables|Default|GetMSS_Music) 0.0))

(event Custom|StartAmbienceSounds_Event
  (bind _fadeinduration (Variables|Default|GetFadeinDuration))
  (Audio|Components|Audio|FadeIn (Variables|Default|GetMSS_Rain_Cricket) _fadeinduration 1.0 0.0 "Linear" :!class /Script/Engine.AudioComponent)
  (Audio|Components|Audio|FadeIn (Variables|Default|GetMSS_Wind) _fadeinduration 1.0 0.0 "Linear" :!class /Script/Engine.AudioComponent))

(event Custom|StopMusic_Event
  (Audio|Components|Audio|FadeOut (Variables|Default|GetMSS_Music) (Variables|Default|GetFadeoutDuration) 0.0 "Linear" :!class /Script/Engine.AudioComponent))

(event Custom|StartMusic_Event
  (Audio|Components|Audio|FadeIn (Variables|Default|GetMSS_Music) (Variables|Default|GetFadeinDuration) 1.0 0.0 "Linear" :!class /Script/Engine.AudioComponent))

(fn ConstructionScript)