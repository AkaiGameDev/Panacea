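; BP_PanaceaGameMode is a game mode that plays a cutscene video when play begins.
; BeginPlay creates a BP_CutsceneWidget if none exists, adds it to the viewport and opens the media source on a media player.
; The player's end-reached event is bound to CloseVideo, which removes the widget from the viewport after a short delay.
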(event Custom|CloseVideo
  (bind _cutscenewidget (Variables|Default|GetCutsceneWidget)
    (:then
      (Utilities|FlowControl|Delay 0.5)
      (Widget|RemovefromParent _cutscenewidget))
    (:else)))

(event EventBeginPlay
  (Variables|Default|GetCutsceneWidget
    (:then
      _)
    (:else
      (bind _returnvalue (UserInterface|CreateWidget "/Game/Blueprints/BP_CutsceneWidget.BP_CutsceneWidget_C" (Game|GetPlayerController 0)))
      (Variables|Default|SetCutsceneWidget _returnvalue)))
  (Media|MediaPlayer|BindEventtoOnEndReached (Variables|Default|GetMediaPlayer) (delegate Custom|CloseVideo))
  (UserInterface|Viewport|AddtoViewport (Variables|Default|GetCutsceneWidget) 0)
  (Media|MediaPlayer|OpenSource (Variables|Default|GetMediaPlayer) (Variables|Default|GetMediaSource)))

(event EventTick
  (params (DeltaSeconds :type Float%20%28single-precision%29)))

(fn ConstructionScript)